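; BP_MusicZone is a test trigger volume that plays safe-zone music while something overlaps it.
; Beginning overlap on the Trigger component spawns a synthwave 2D sound and fades it in, and ending overlap fades it out.
; Neither handler filters the overlapping actor, so each new overlap spawns another sound and replaces the stored reference.
; A battle-music spawn and fade-in branch exists but is unconnected.
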(event OnComponentBeginOverlap(Trigger)
  (params (OverlappedComponent :type Primitive%20Component%20Object%20Reference) (OtherActor :type Actor%20Object%20Reference) (OtherComp :type Primitive%20Component%20Object%20Reference) (OtherBodyIndex :type Integer) (bFromSweep :type Boolean) (SweepResult :type Hit%20Result%20Structure%20%28by%20ref%29))
  (if true
    (bind _returnvalue (Audio|SpawnSound2D "/Game/MusicSound/Alexi_Action-I_Am_a_Robot__Dark_Synthwave_.Alexi_Action-I_Am_a_Robot__Dark_Synthwave_" 1.0 1.0 0.0 0))
    (bind _output_get (Variables|Default|SetSafeZoneMusic _returnvalue))
    (Audio|Components|Audio|FadeIn _output_get 1.0 1.0 0.0 "Linear" :!class /Script/Engine.AudioComponent)))

(event OnComponentEndOverlap(Trigger)
  (params (OverlappedComponent :type Primitive%20Component%20Object%20Reference) (OtherActor :type Actor%20Object%20Reference) (OtherComp :type Primitive%20Component%20Object%20Reference) (OtherBodyIndex :type Integer))
  (if true
    (bind _safezonemusic (Variables|Default|GetSafeZoneMusic)
      (:then
        (Audio|Components|Audio|FadeOut _safezonemusic 1.0 0.0 "Linear" :!class /Script/Engine.AudioComponent))
      (:else))))

(event Collision|EventActorBeginOverlap
  (params (OtherActor :type Actor%20Object%20Reference)))

(event EventTick
  (params (DeltaSeconds :type Float%20%28single-precision%29)))

(event EventBeginPlay)

(fn ConstructionScript)