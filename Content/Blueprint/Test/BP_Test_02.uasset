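; Test ammo pickup actor that refills the first-person character's SMG and shotgun reserves (ChargeurSMG, ChargeurShotgun).
; BeginPlay caches the player character, and any Collision overlap modifies that reference without checking the overlapping actor.
; Threshold branches add ammo or cap the shotgun, but high SMG ammo below its upper limit resets to zero, skipping shotgun refill.
; The actor destroys itself only on some branches; an unconnected combined check remains unused.
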(event OnComponentBeginOverlap(Collision)
  (params (OverlappedComponent :type Primitive%20Component%20Object%20Reference) (OtherActor :type Actor%20Object%20Reference) (OtherComp :type Primitive%20Component%20Object%20Reference) (OtherBodyIndex :type Integer) (bFromSweep :type Boolean) (SweepResult :type Hit%20Result%20Structure%20%28by%20ref%29))
  (bind _as_bp_first_person_character (Variables|Default|GetAs%20BP%20First%20Person%20Character))
  (bind _as_bp_first_person_character_2 (Variables|Default|GetAs%20BP%20First%20Person%20Character))
  (if (<= (Variables|/Game/Player/FirstPerson/Blueprints/BP_FirstPersonCharacter.BP_FirstPersonCharacter_C|GetChargeur_SMG _as_bp_first_person_character_2) 1e+02)
    (Variables|/Game/Player/FirstPerson/Blueprints/BP_FirstPersonCharacter.BP_FirstPersonCharacter_C|SetChargeur_SMG _as_bp_first_person_character_2 (+ (Variables|/Game/Player/FirstPerson/Blueprints/BP_FirstPersonCharacter.BP_FirstPersonCharacter_C|GetChargeur_SMG _as_bp_first_person_character_2) (Variables|Default|GetQte_de_munitions_SMG)))
    (if (<= (Variables|/Game/Player/FirstPerson/Blueprints/BP_FirstPersonCharacter.BP_FirstPersonCharacter_C|GetChargeur_Shotgun _as_bp_first_person_character) 2e+01)
      (Variables|/Game/Player/FirstPerson/Blueprints/BP_FirstPersonCharacter.BP_FirstPersonCharacter_C|SetChargeur_Shotgun _as_bp_first_person_character (+ (Variables|/Game/Player/FirstPerson/Blueprints/BP_FirstPersonCharacter.BP_FirstPersonCharacter_C|GetChargeur_Shotgun _as_bp_first_person_character) (Variables|Default|GetQte_de_munitions_Shotgun)))
      (Actor|DestroyActor :!label _label)
      (elif (and (< (Variables|/Game/Player/FirstPerson/Blueprints/BP_FirstPersonCharacter.BP_FirstPersonCharacter_C|GetChargeur_Shotgun _as_bp_first_person_character) 3e+01) (> (Variables|/Game/Player/FirstPerson/Blueprints/BP_FirstPersonCharacter.BP_FirstPersonCharacter_C|GetChargeur_Shotgun _as_bp_first_person_character) 2e+01))
        (Variables|/Game/Player/FirstPerson/Blueprints/BP_FirstPersonCharacter.BP_FirstPersonCharacter_C|SetChargeur_Shotgun _as_bp_first_person_character 3e+01)
        (goto _label)))
    (elif (and (< (Variables|/Game/Player/FirstPerson/Blueprints/BP_FirstPersonCharacter.BP_FirstPersonCharacter_C|GetChargeur_SMG _as_bp_first_person_character_2) 1.5e+02) (> (Variables|/Game/Player/FirstPerson/Blueprints/BP_FirstPersonCharacter.BP_FirstPersonCharacter_C|GetChargeur_SMG _as_bp_first_person_character_2) 1e+02))
      (Variables|/Game/Player/FirstPerson/Blueprints/BP_FirstPersonCharacter.BP_FirstPersonCharacter_C|SetChargeur_SMG (Variables|Default|GetAs%20BP%20First%20Person%20Character) 0.0)
      (Actor|DestroyActor))))

(event EventBeginPlay
  (bind _asbp_first_person_character (Utilities|Casting|CastToBP_FirstPersonCharacter (Game|GetPlayerCharacter 0)))
  (Variables|Default|SetAs%20BP%20First%20Person%20Character _asbp_first_person_character))

(fn ConstructionScript)