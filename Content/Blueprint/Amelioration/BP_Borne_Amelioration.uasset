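; Upgrade terminal Blueprint that toggles an on-screen widget when its Interaction event fires.
; BeginPlay creates a WB_Test widget once and caches it along with the player's BP_FirstPersonCharacter.
; Each Interaction reads the character's IsLooking flag to add or remove the widget, then flips that flag and the mouse cursor visibility to match.
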(event EventBeginPlay
  (bind _returnvalue (UserInterface|CreateWidget "/Game/UI/Widget/WB_Test.WB_Test_C"))
  (Variables|Default|SetNewVar _returnvalue)
  (bind _asbp_first_person_character (Utilities|Casting|CastToBP_FirstPersonCharacter (Game|GetPlayerCharacter 0)))
  (Variables|Default|SetAs%20BP%20First%20Person%20Character _asbp_first_person_character))

(event EventInteraction
  (bind _returnvalue (Game|GetPlayerController 0))
  (if (not (Variables|/Game/Player/FirstPerson/Blueprints/BP_FirstPersonCharacter.BP_FirstPersonCharacter_C|GetIs_Looking (Variables|Default|GetAs%20BP%20First%20Person%20Character)))
    (UserInterface|Viewport|AddtoViewport (Variables|Default|GetNewVar) 0)
    (Variables|/Game/Player/FirstPerson/Blueprints/BP_FirstPersonCharacter.BP_FirstPersonCharacter_C|SetIs_Looking (Variables|Default|GetAs%20BP%20First%20Person%20Character) true)
    (Variables|/Script/Engine.PlayerController|SetbShowMouseCursor _returnvalue true)
    (else
      (Widget|RemovefromParent (Variables|Default|GetNewVar))
      (Variables|/Game/Player/FirstPerson/Blueprints/BP_FirstPersonCharacter.BP_FirstPersonCharacter_C|SetIs_Looking (Variables|Default|GetAs%20BP%20First%20Person%20Character) false)
      (Variables|/Script/Engine.PlayerController|SetbShowMouseCursor _returnvalue false))))

(fn ConstructionScript)