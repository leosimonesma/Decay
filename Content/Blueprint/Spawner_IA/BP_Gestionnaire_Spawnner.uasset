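; Spawner manager that triggers a wave of AI spawns once, when the player overlaps its box.
; On BeginPlay it pre-rolls a random spawner index for each spawn in the Game Instance's count and gathers the BP_Spawner actors sharing its ID.
; The one-shot overlap then runs those indices, re-querying each spawner until its point differs from the last one used before spawning there.
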(event OnComponentBeginOverlap(Box)
  (params (OverlappedComponent :type Primitive%20Component%20Object%20Reference) (OtherActor :type Actor%20Object%20Reference) (OtherComp :type Primitive%20Component%20Object%20Reference) (OtherBodyIndex :type Integer) (bFromSweep :type Boolean) (SweepResult :type Hit%20Result%20Structure%20%28by%20ref%29))
  ;[1 1 1] Declencher le spawn
  (if (== OtherActor (Game|GetPlayerCharacter 0))
    (Utilities|FlowControl|DoOnce false
      (:Completed
        (CallFunction|Spawn)))))

(event Custom|Spawn
  ;[1 1 1] Déclenchement des spawn en do once pour empecher le player de faire spawn a l'infini
  (Development|PrintString "Hello")
  (for _array_element (Variables|Static|GetTable_Of_Spawn)
    (bind _next_point (Default|Spawning (Utilities|Array|Get(acopy) (Variables|Static|GetRef_Spawner) _array_element) :!label _label))
    (if (Class|KismetMathLibrary|EqualExactlyVectorVector _next_point (Variables|Default|GetLast_Point))
      (goto _label)
      (else
        (bind _output_get (Variables|Default|SetLast_Point _next_point))
        (Default|Spawn (Utilities|Array|Get(acopy) (Variables|Static|GetRef_Spawner) _array_element) _output_get)))))

(event EventBeginPlay
  ;[1 1 1] Récuperation de tous les spawners et set dans un tableau pour ensuite choisir aléatoirement un spawn dans pour chaque ennemis qui doit apparaitre (déterminé grace a une variable
  (Variables|Static|SetAs%20BP%20Game%20Instance (.AsBP%20Game%20Instance (Utilities|Casting|CastToBP_Game_Instance (Game|GetGameInstance))))
  (bind _asbp_first_person_character (Utilities|Casting|CastToBP_FirstPersonCharacter (Game|GetPlayerCharacter 0)))
  (Variables|Static|SetAs%20BP%20First%20Person%20Character _asbp_first_person_character)
  (bind _output_get (Variables|InstanceEditable|SetNb_Of_Spawn (Variables|/Game/Blueprint/GameInstance/BP_Game_Instance.BP_Game_Instance_C|GetNb_De_Spawn (Variables|Static|GetAs%20BP%20Game%20Instance))))
  (if (!= (Variables|InstanceEditable|GetNb_Of_Spawn) 0) :!label _label
    (Utilities|Array|Add (Variables|Static|GetTable_Of_Spawn) (Math|Random|RandomInteger (Variables|InstanceEditable|GetMax_Random_Spawner)))
    (Math|Integer|DecrementInt _output_get
      (:%20%20
        (goto _label)))
    (else
      (bind _outactors (Actor|GetAllActorsOfClass "/Game/Blueprint/Spawner_IA/BP_Spawner.BP_Spawner_C"))
      (for _array_element _outactors
        (if (== (Variables|/Game/Blueprint/Spawner_IA/BP_Spawner.BP_Spawner_C|GetID _array_element) (Variables|InstanceEditable|GetID))
          (Utilities|Array|Add (Variables|Static|GetRef_Spawner) _array_element))))))

(fn ConstructionScript)