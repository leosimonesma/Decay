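; Start-game trigger actor that fires a randomized set of spawns from the level's BP_Spawner actors.
; On BeginPlay it caches the player character, fills TableOfSpawn with NBOfSpawn random indices, then collects every spawner into RefSpawner.
; The first Box overlap, unfiltered by actor, calls Spawn on the spawner at each stored index, guarded by DoOnce.
; The random range is hardcoded to three spawners, regardless of how many are found.
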(event OnComponentBeginOverlap(Box)
  (params (OverlappedComponent :type Primitive%20Component%20Object%20Reference) (OtherActor :type Actor%20Object%20Reference) (OtherComp :type Primitive%20Component%20Object%20Reference) (OtherBodyIndex :type Integer) (bFromSweep :type Boolean) (SweepResult :type Hit%20Result%20Structure%20%28by%20ref%29))
  (Utilities|FlowControl|DoOnce false
    (:Completed
      (for _array_element (Variables|Default|GetTable_Of_Spawn)
        (Default|Spawn (Utilities|Array|Get(acopy) (Variables|Default|GetRef_Spawner) _array_element))))))

(event EventBeginPlay
  (bind _asbp_first_person_character (Utilities|Casting|CastToBP_FirstPersonCharacter (Game|GetPlayerCharacter 0)))
  (Variables|Default|SetAs%20BP%20First%20Person%20Character _asbp_first_person_character)
  (if (!= (Variables|Default|GetNB_Of_Spawn) 0) :!label _label
    (Utilities|Array|Add (Variables|Default|GetTable_Of_Spawn) (Math|Random|RandomInteger 3))
    (Math|Integer|DecrementInt (Variables|Default|GetNB_Of_Spawn)
      (:%20%20
        (goto _label)))
    (else
      (bind _outactors (Actor|GetAllActorsOfClass "/Game/Blueprint/Spawner_IA/BP_Spawner.BP_Spawner_C"))
      (for _array_element _outactors
        (Utilities|Array|Add (Variables|Default|GetRef_Spawner) _array_element)
        (Development|PrintString "Hello")))))

(fn ConstructionScript)