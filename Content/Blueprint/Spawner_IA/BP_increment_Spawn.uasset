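; BP_increment_Spawn is a trigger box that tracks living enemies and raises spawn counts as areas are entered.
; The just_spawned and Die events adjust the enemy counter, which is printed every tick for debugging.
; When the player overlaps the box with no enemies left, it calls the door-open event and plays a clear sound.
; A DoOnce on overlap adds a small random amount to the Game Instance's spawn count.
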(event OnComponentBeginOverlap(Box)
  (params (OverlappedComponent :type Primitive%20Component%20Object%20Reference) (OtherActor :type Actor%20Object%20Reference) (OtherComp :type Primitive%20Component%20Object%20Reference) (OtherBodyIndex :type Integer) (bFromSweep :type Boolean) (SweepResult :type Hit%20Result%20Structure%20%28by%20ref%29))
  (bind _as_bp_game_instance (Variables|Static|GetAs%20BP%20Game%20Instance))
  ;[1 1 1] incrementation du nombre de spawn quand on rentre dedans
  (if (and (<= (Variables|Default|GetNb_Ennemy) 0) (== OtherActor (Game|GetPlayerCharacter 0)))
    (Default|CallOpenDoor)
    (Audio|PlaySound2D "/Game/MusicSound/SFX/Clear.Clear" 2.0 1.0 0.0 0 0))
  (Utilities|FlowControl|DoOnce false
    (:Completed
      (Variables|/Game/Blueprint/GameInstance/BP_Game_Instance.BP_Game_Instance_C|SetNb_De_Spawn _as_bp_game_instance (+ (Variables|/Game/Blueprint/GameInstance/BP_Game_Instance.BP_Game_Instance_C|GetNb_De_Spawn _as_bp_game_instance) (Math|Random|RandomIntegerinRange 2 4))))))

(event Custom|Die
  (Math|Integer|DecrementInt (Variables|Default|GetNb_Ennemy)))

(event Custom|just_spawned
  (bind _result (Math|Integer|IncrementInt (Variables|Default|GetNb_Ennemy))
    (:%20%20
      (Variables|Default|SetNb_Ennemy _result))))

(event EventTick
  (params (DeltaSeconds :type Float%20%28single-precision%29))
  (Development|PrintString (Utilities|String|ToString(Integer) (Variables|Default|GetNb_Ennemy)) true true "(R=0.000000,G=0.660000,B=1.000000,A=1.000000)" 0.0))

(event EventBeginPlay
  (Variables|Static|SetAs%20BP%20Game%20Instance (.AsBP%20Game%20Instance (Utilities|Casting|CastToBP_Game_Instance (Game|GetGameInstance)))))

(fn ConstructionScript)