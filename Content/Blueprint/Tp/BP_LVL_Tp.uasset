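; Elevator level exit that shows the current floor and, when used, advances the run to a randomly picked level.
; It stays locked, playing a denied sound, until the RefIncrementSpawn event unlocks it and starts a flickering light.
; Interaction animates the button, shows a transition widget, increments the Game Instance floor and opens the level.
; Game Instance counters drive a reroll that prevents the same level appearing three times in a row.
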(event OnComponentBeginOverlap(Box1)
  (params (OverlappedComponent :type Primitive%20Component%20Object%20Reference) (OtherActor :type Actor%20Object%20Reference) (OtherComp :type Primitive%20Component%20Object%20Reference) (OtherBodyIndex :type Integer) (bFromSweep :type Boolean) (SweepResult :type Hit%20Result%20Structure%20%28by%20ref%29))
  (if (== OtherActor (Game|GetPlayerCharacter 0))
    (if (not (Variables|Default|GetLock))
      (Rendering|SetVisibility (Variables|Default|GetWidget) false false))))

(event OnComponentEndOverlap(Box1)
  (params (OverlappedComponent :type Primitive%20Component%20Object%20Reference) (OtherActor :type Actor%20Object%20Reference) (OtherComp :type Primitive%20Component%20Object%20Reference) (OtherBodyIndex :type Integer))
  (if (== OtherActor (Game|GetPlayerCharacter 0))
    (Rendering|SetVisibility (Variables|Default|GetWidget) false false)))

(event Custom|Open_The_Lock
  (Variables|Default|SetLock false)
  (bind _flickering (Timeline|Flickering Play)
    (:Update
      (Rendering|Components|Light|SetIntensity (Variables|Default|GetPointLight) (* _flickering 1e+01)))))

(event EventTick
  (params (DeltaSeconds :type Float%20%28single-precision%29))
  (Transformation|SetWorldRotation (Variables|Default|GetWidget) (Math|Rotator|FindLookatRotation (Transformation|GetWorldLocation (Variables|Default|GetElevator%20Button)) (Transformation|GetWorldLocation (Variables|/Script/Engine.Character|GetMesh (Variables|Default|GetAs%20BP%20First%20Person%20Character)))) false false))

(event EventBeginPlay
  (Variables|Default|SetLock true)
  (bind _asbp_game_instance (Utilities|Casting|CastToBP_Game_Instance (Game|GetGameInstance)))
  (Variables|Default|SetAs%20BP%20Game%20Instance _asbp_game_instance)
  (bind _asbp_first_person_character (Utilities|Casting|CastToBP_FirstPersonCharacter (Game|GetPlayerCharacter 0)))
  (Variables|Default|SetAs%20BP%20First%20Person%20Character _asbp_first_person_character)
  (Rendering|SetVisibility (Variables|Default|GetWidget) false false)
  (EventDispatchers|BindEventtoOpenDoor (Variables|Default|GetRef_increment_spawn) (delegate Custom|Open_The_Lock))
  (Actor|GetAllActorsOfClass "/Game/Blueprint/Spawner_IA/BP_Gestionnaire_Spawnner.BP_Gestionnaire_Spawnner_C")
  (Variables|Default|SetCurrent%20Floor (Utilities|String|ToString(Integer) (Variables|/Game/Blueprint/GameInstance/BP_Game_Instance.BP_Game_Instance_C|GetFloor (Variables|Default|GetAs%20BP%20Game%20Instance))))
  (Rendering|Components|TextRender|SetText (Variables|Default|GetTextRender) (Utilities|Text|FormatText "F {Floor}" (Variables|Default|GetCurrent%20Floor)))
  (bind _returnvalue (UserInterface|CreateWidget "/Game/UI/Widget/WB_Transition.WB_Transition_C"))
  (Variables|Default|SetTransition_Ref _returnvalue))

(event EventInteraction
  (bind _as_bp_game_instance (Variables|Default|GetAs%20BP%20Game%20Instance))
  (bind _as_bp_game_instance_2 (Variables|Default|GetAs%20BP%20Game%20Instance))
  ;[1 1 1] Change lvl en étant sur que l'on ne peut pas tomber 3 fois de suite sur le meme lvl
  (if (not (Variables|Default|GetLock))
    (Audio|PlaySound2D "/Game/MusicSound/SFX/Button_Click.Button_Click" 1.0 1.0 0.0 0 0)
    (Transformation|SetRelativeLocation (Variables|Default|GetElevator%20Button) "5.000000,0.000000,0.000000" false false)
    (Utilities|FlowControl|Delay 1.0)
    (Transformation|SetRelativeLocation (Variables|Default|GetElevator%20Button) "-5.000000,0.000000,0.000000" false false)
    (UserInterface|Viewport|AddtoViewport (Variables|Default|GetTransition_Ref) 0)
    (Utilities|FlowControl|Delay 2.0)
    (Math|Integer|IncrementInt (Variables|/Game/Blueprint/GameInstance/BP_Game_Instance.BP_Game_Instance_C|GetFloor (Variables|Default|GetAs%20BP%20Game%20Instance))
      (:%20%20
        (bind _output_get (Variables|/Game/Blueprint/GameInstance/BP_Game_Instance.BP_Game_Instance_C|SetLast_LVL _as_bp_game_instance (.OutItem (Utilities|Array|Random (Variables|Default|GetLevel_ref))) :!label _label))
        (if (== _output_get (Variables|/Game/Blueprint/GameInstance/BP_Game_Instance.BP_Game_Instance_C|GetCurrent_LVL _as_bp_game_instance))
          (Math|Integer|IncrementInt (Variables|/Game/Blueprint/GameInstance/BP_Game_Instance.BP_Game_Instance_C|GetCompteur _as_bp_game_instance_2)
            (:%20%20
              _))
          (else
            (Variables|/Game/Blueprint/GameInstance/BP_Game_Instance.BP_Game_Instance_C|SetCurrent_LVL _as_bp_game_instance _output_get)
            (Variables|/Game/Blueprint/GameInstance/BP_Game_Instance.BP_Game_Instance_C|SetCompteur _as_bp_game_instance_2 0)))
        (if (>= (Variables|/Game/Blueprint/GameInstance/BP_Game_Instance.BP_Game_Instance_C|GetCompteur _as_bp_game_instance_2) 2)
          (goto _label)
          (else
            (Game|OpenLevel(byObjectReference) (Variables|/Game/Blueprint/GameInstance/BP_Game_Instance.BP_Game_Instance_C|GetCurrent_LVL (Variables|Default|GetAs%20BP%20Game%20Instance)))))))
    (else
      (Audio|PlaySound2D "/Game/MusicSound/SFX/Access_Denied_Sound_Effect.Access_Denied_Sound_Effect" 2.0 1.0 0.0 0 0))))

(fn ConstructionScript)