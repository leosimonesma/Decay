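; BP_Restoration is a one-time restoration trigger that refills the player's health and ammunition.
; On BeginPlay it caches BP_Game_Instance, and a box overlap by the player copies the stored maximums into current HP plus SMG and shotgun magazine and reserve ammo.
; A DoOnce runs before the player check, so the first overlap by any actor uses up the trigger.
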(event OnComponentBeginOverlap(Box)
  (params (OverlappedComponent :type Primitive%20Component%20Object%20Reference) (OtherActor :type Actor%20Object%20Reference) (OtherComp :type Primitive%20Component%20Object%20Reference) (OtherBodyIndex :type Integer) (bFromSweep :type Boolean) (SweepResult :type Hit%20Result%20Structure%20%28by%20ref%29))
  (bind _as_bp_game_instance (Variables|Default|GetAs%20BP%20Game%20Instance))
  (Utilities|FlowControl|DoOnce false
    (:Completed
      (if (== OtherActor (Game|GetPlayerCharacter 0))
        (Variables|/Game/Blueprint/GameInstance/BP_Game_Instance.BP_Game_Instance_C|SetPlayer_HP _as_bp_game_instance (Variables|/Game/Blueprint/GameInstance/BP_Game_Instance.BP_Game_Instance_C|GetMax_Health _as_bp_game_instance))
        (Variables|/Game/Blueprint/GameInstance/BP_Game_Instance.BP_Game_Instance_C|SetGun_reserve_SMG _as_bp_game_instance (Variables|/Game/Blueprint/GameInstance/BP_Game_Instance.BP_Game_Instance_C|GetGun_Max_reserve_SMG _as_bp_game_instance))
        (Variables|/Game/Blueprint/GameInstance/BP_Game_Instance.BP_Game_Instance_C|SetGun_reserve_Shotgun _as_bp_game_instance (Variables|/Game/Blueprint/GameInstance/BP_Game_Instance.BP_Game_Instance_C|GetGun_Max_reserve_Shotgun _as_bp_game_instance))
        (Variables|/Game/Blueprint/GameInstance/BP_Game_Instance.BP_Game_Instance_C|SetGun_Munitions_Shotgun _as_bp_game_instance (Variables|/Game/Blueprint/GameInstance/BP_Game_Instance.BP_Game_Instance_C|GetGun_Max_Munitions_Shotgun _as_bp_game_instance))
        (Variables|/Game/Blueprint/GameInstance/BP_Game_Instance.BP_Game_Instance_C|SetGun_Muntions_SMG _as_bp_game_instance (Variables|/Game/Blueprint/GameInstance/BP_Game_Instance.BP_Game_Instance_C|GetGun_Max_Munitions_SMG _as_bp_game_instance))))))

(event EventBeginPlay
  (bind _asbp_game_instance (Utilities|Casting|CastToBP_Game_Instance (Game|GetGameInstance)))
  (Variables|Default|SetAs%20BP%20Game%20Instance _asbp_game_instance))

(fn ConstructionScript)