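; Behavior tree task that checks whether the first player's controller has line of sight to the AI-controlled pawn.
; On AI execution it calls LineOfSightTo on that pawn, passing the forward vector of the SelfRef blackboard actor as the view point.
; The task finishes with success when the pawn is visible and failure otherwise, printing a debug string in either case.
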(event EventReceiveExecuteAI
  (params (OwnerController :type AI%20Controller%20Object%20Reference) (ControlledPawn :type Pawn%20Object%20Reference))
  (if (Controller|LineOfSightTo (Game|GetPlayerController (Variables|/Script/Engine.Pawn|GetPlayerState (Game|GetPlayerCharacter 0))) ControlledPawn (Transformation|GetActorForwardVector (AI|BehaviorTree|GetBlackboardValueasActor (Variables|Default|GetSelf_Ref))) false)
    (Development|PrintString "Hello")
    (AI|BehaviorTree|FinishExecute true)
    (else
      (Development|PrintString "Nope")
      (AI|BehaviorTree|FinishExecute false))))