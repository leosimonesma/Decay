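; Boss room door that starts locked with a red lamp and unlocks when an event bound through RefIncrementSpawn fires.
; Unlocking turns the lamp green and removes a plane and point light.
; While unlocked, player overlap with the door trigger plays a timeline that slides both leaves apart with sound, reversing on exit.
; A separate closed trigger sets the lock again when the player enters it, disabling further door movement triggers.
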(event OnComponentBeginOverlap(Closed_Trigger)
  (params (OverlappedComponent :type Primitive%20Component%20Object%20Reference) (OtherActor :type Actor%20Object%20Reference) (OtherComp :type Primitive%20Component%20Object%20Reference) (OtherBodyIndex :type Integer) (bFromSweep :type Boolean) (SweepResult :type Hit%20Result%20Structure%20%28by%20ref%29))
  (if (== OtherActor (Game|GetPlayerCharacter 0))
    (Variables|Default|SetLock true)))

(event OnComponentBeginOverlap(Door_Trigger)
  (params (OverlappedComponent :type Primitive%20Component%20Object%20Reference) (OtherActor :type Actor%20Object%20Reference) (OtherComp :type Primitive%20Component%20Object%20Reference) (OtherBodyIndex :type Integer) (bFromSweep :type Boolean) (SweepResult :type Hit%20Result%20Structure%20%28by%20ref%29))
  (if (== OtherActor (Game|GetPlayerCharacter 0))
    (if (not (Variables|Default|GetLock))
      (Audio|Components|Audio|Play (Variables|Default|GetDoor_SFX) 0.0)
      (bind _door_open (Timeline|Timeline Play)
        (:Update
          (Transformation|SetRelativeLocation (Variables|Default|GetL_Door) (Math|Vector|Lerp(Vector) "0, 0, 0" "0.000000,150.000000,0.000000" _door_open) false false)
          (Transformation|SetRelativeLocation (Variables|Default|GetR_Door) (Math|Vector|Lerp(Vector) "0, 0, 0" "0.000000,-150.000000,0.000000" _door_open) false false))))))

(event OnComponentEndOverlap(Door_Trigger)
  (params (OverlappedComponent :type Primitive%20Component%20Object%20Reference) (OtherActor :type Actor%20Object%20Reference) (OtherComp :type Primitive%20Component%20Object%20Reference) (OtherBodyIndex :type Integer))
  (if (== OtherActor (Game|GetPlayerCharacter 0))
    (if (not (Variables|Default|GetLock))
      (Audio|Components|Audio|Play (Variables|Default|GetDoor_SFX) 0.0)
      (bind _door_open (Timeline|Timeline Reverse)
        (:Update
          (Transformation|SetRelativeLocation (Variables|Default|GetL_Door) (Math|Vector|Lerp(Vector) "0, 0, 0" "0.000000,150.000000,0.000000" _door_open) false false)
          (Transformation|SetRelativeLocation (Variables|Default|GetR_Door) (Math|Vector|Lerp(Vector) "0, 0, 0" "0.000000,-150.000000,0.000000" _door_open) false false))))))

(event Custom|Open_The_Lock
  ;[1 1 1] Being_play
  (Variables|Default|SetLock false)
  (Rendering|Material|SetVectorParameterValueonMaterials (Variables|Default|GetLampe) "Color" "0.000000,1.000000,0.000000")
  (Components|DestroyComponent (Variables|Default|GetPlane)))

(event EventBeginPlay
  ;[1 1 1] Being_play
  (Variables|Default|SetLock true)
  (Rendering|Material|SetVectorParameterValueonMaterials (Variables|Default|GetLampe) "Color" "1.000000,0.000000,0.000000")
  (EventDispatchers|BindEventtoOpenDoor (Variables|Default|GetRef_Increment_spawn) (delegate Custom|Open_The_Lock)))

(fn ConstructionScript)