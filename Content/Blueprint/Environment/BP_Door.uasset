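; BP_Door is an automatic double sliding door that opens when the player approaches and closes when they leave.
; A Box trigger reacts only to the player character, plays the door sound and runs a timeline forward on entry or in reverse on exit.
; The timeline's DoorOpen track lerps the left and right panels apart along their local Y axis in opposite directions.
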(event OnComponentBeginOverlap(Box)
  (params (OverlappedComponent :type Primitive%20Component%20Object%20Reference) (OtherActor :type Actor%20Object%20Reference) (OtherComp :type Primitive%20Component%20Object%20Reference) (OtherBodyIndex :type Integer) (bFromSweep :type Boolean) (SweepResult :type Hit%20Result%20Structure%20%28by%20ref%29))
  (if (== OtherActor (Game|GetPlayerCharacter 0))
    (Audio|Components|Audio|Play (Variables|Default|GetDoor_SFX) 0.0)
    (bind _door_open (Timeline|Timeline Play)
      (:Update
        (Transformation|SetRelativeLocation (Variables|Default|GetL_Door) (Math|Vector|Lerp(Vector) "0, 0, 0" "0.000000,150.000000,0.000000" _door_open) false false)
        (Transformation|SetRelativeLocation (Variables|Default|GetR_Door) (Math|Vector|Lerp(Vector) "0, 0, 0" "0.000000,-150.000000,0.000000" _door_open) false false)))))

(event OnComponentEndOverlap(Box)
  (params (OverlappedComponent :type Primitive%20Component%20Object%20Reference) (OtherActor :type Actor%20Object%20Reference) (OtherComp :type Primitive%20Component%20Object%20Reference) (OtherBodyIndex :type Integer))
  (if (== OtherActor (Game|GetPlayerCharacter 0))
    (Audio|Components|Audio|Play (Variables|Default|GetDoor_SFX) 0.0)
    (bind _door_open (Timeline|Timeline Reverse)
      (:Update
        (Transformation|SetRelativeLocation (Variables|Default|GetL_Door) (Math|Vector|Lerp(Vector) "0, 0, 0" "0.000000,150.000000,0.000000" _door_open) false false)
        (Transformation|SetRelativeLocation (Variables|Default|GetR_Door) (Math|Vector|Lerp(Vector) "0, 0, 0" "0.000000,-150.000000,0.000000" _door_open) false false)))))

(fn ConstructionScript)