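; BP_Heal_Drop is a pickup actor that restores the player's Pv (health) and then destroys itself.
; On BeginPlay it caches the first-person character and records that character's current Pv as the maximum.
; Any overlap with its Collision component, without checking the overlapping actor, adds QteHeal to the player's Pv, capped at that recorded maximum.
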(event OnComponentBeginOverlap(Collision)
  (params (OverlappedComponent :type Primitive%20Component%20Object%20Reference) (OtherActor :type Actor%20Object%20Reference) (OtherComp :type Primitive%20Component%20Object%20Reference) (OtherBodyIndex :type Integer) (bFromSweep :type Boolean) (SweepResult :type Hit%20Result%20Structure%20%28by%20ref%29))
  (bind _as_bp_first_person_character (Variables|Default|GetAs%20BP%20First%20Person%20Character))
  (if (> (Variables|/Game/Player/FirstPerson/Blueprints/BP_FirstPersonCharacter.BP_FirstPersonCharacter_C|GetPv (Variables|Default|GetAs%20BP%20First%20Person%20Character)) (- (Variables|Default|GetPV_Max) (Variables|Default|GetQte_Heal)))
    (Variables|/Game/Player/FirstPerson/Blueprints/BP_FirstPersonCharacter.BP_FirstPersonCharacter_C|SetPv _as_bp_first_person_character (Variables|Default|GetPV_Max))
    (Actor|DestroyActor)
    (else
      (Variables|/Game/Player/FirstPerson/Blueprints/BP_FirstPersonCharacter.BP_FirstPersonCharacter_C|SetPv _as_bp_first_person_character (+ (Variables|/Game/Player/FirstPerson/Blueprints/BP_FirstPersonCharacter.BP_FirstPersonCharacter_C|GetPv _as_bp_first_person_character) (Variables|Default|GetQte_Heal)))
      (Actor|DestroyActor))))

(event EventBeginPlay
  (bind _asbp_first_person_character (Utilities|Casting|CastToBP_FirstPersonCharacter (Game|GetPlayerCharacter 0)))
  (bind _output_get (Variables|Default|SetAs%20BP%20First%20Person%20Character _asbp_first_person_character))
  (Variables|Default|SetPV_Max (Variables|/Game/Player/FirstPerson/Blueprints/BP_FirstPersonCharacter.BP_FirstPersonCharacter_C|GetPv _output_get)))

(fn ConstructionScript)