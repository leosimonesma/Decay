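; Ammo drop pickup that refills the player's SMG and shotgun reserves when the player character overlaps it.
; Overlap plays a grab sound and shows a WB_Ammo_Gain widget.
; A nested branch chain compares each reserve in BP_Game_Instance to its thresholds, then adds a set amount or fills to max.
; Every outcome destroys the pickup and calls SetReserve on the character, even with full reserves.
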(event OnComponentBeginOverlap(Collision)
  (params (OverlappedComponent :type Primitive%20Component%20Object%20Reference) (OtherActor :type Actor%20Object%20Reference) (OtherComp :type Primitive%20Component%20Object%20Reference) (OtherBodyIndex :type Integer) (bFromSweep :type Boolean) (SweepResult :type Hit%20Result%20Structure%20%28by%20ref%29))
  (bind _as_bp_game_instance (Variables|Static|GetAs%20BP%20Game%20Instance))
  (bind _as_bp_game_instance_2 (Variables|Static|GetAs%20BP%20Game%20Instance))
  (bind _as_bp_game_instance_3 (Variables|Static|GetAs%20BP%20Game%20Instance))
  (bind _as_bp_game_instance_4 (Variables|Static|GetAs%20BP%20Game%20Instance))
  (bind _as_bp_game_instance_5 (Variables|Static|GetAs%20BP%20Game%20Instance))
  (bind _as_bp_game_instance_6 (Variables|Static|GetAs%20BP%20Game%20Instance))
  (bind _as_bp_game_instance_7 (Variables|Static|GetAs%20BP%20Game%20Instance))
  (bind _as_bp_game_instance_8 (Variables|Static|GetAs%20BP%20Game%20Instance))
  (bind _as_bp_game_instance_9 (Variables|Static|GetAs%20BP%20Game%20Instance))
  (bind _as_bp_game_instance_10 (Variables|Static|GetAs%20BP%20Game%20Instance))
  (bind _as_bp_game_instance_11 (Variables|Static|GetAs%20BP%20Game%20Instance))
  (bind _as_bp_game_instance_12 (Variables|Static|GetAs%20BP%20Game%20Instance))
  (bind _as_bp_game_instance_13 (Variables|Static|GetAs%20BP%20Game%20Instance))
  (bind _as_bp_game_instance_14 (Variables|Static|GetAs%20BP%20Game%20Instance))
  (bind _as_bp_game_instance_15 (Variables|Static|GetAs%20BP%20Game%20Instance))
  (bind _as_bp_game_instance_16 (Variables|Static|GetAs%20BP%20Game%20Instance))
  (bind _as_bp_game_instance_17 (Variables|Static|GetAs%20BP%20Game%20Instance))
  (bind _gun_max_munitions_shotgun (Variables|/Game/Blueprint/GameInstance/BP_Game_Instance.BP_Game_Instance_C|GetGun_Max_Munitions_Shotgun _as_bp_game_instance_10))
  (bind _gun_max_reserve_shotgun (Variables|/Game/Blueprint/GameInstance/BP_Game_Instance.BP_Game_Instance_C|GetGun_Max_reserve_Shotgun _as_bp_game_instance))
  (bind _gun_max_munitions_shotgun_2 (Variables|/Game/Blueprint/GameInstance/BP_Game_Instance.BP_Game_Instance_C|GetGun_Max_Munitions_Shotgun _as_bp_game_instance))
  (bind _gun_max_munitions_smg (Variables|/Game/Blueprint/GameInstance/BP_Game_Instance.BP_Game_Instance_C|GetGun_Max_Munitions_SMG _as_bp_game_instance_3))
  (bind _gun_max_munitions_smg_2 (Variables|/Game/Blueprint/GameInstance/BP_Game_Instance.BP_Game_Instance_C|GetGun_Max_Munitions_SMG _as_bp_game_instance_10))
  ;[1 1 1] Si les deux armes on été utilisées
  (if (== OtherActor (Variables|Static|GetAs%20BP%20First%20Person%20Character))
    (Audio|PlaySound2D "/Game/MusicSound/SFX/Ammo_Grab.Ammo_Grab" 1.0 1.0 0.0 0 0)
    (bind _returnvalue (UserInterface|CreateWidget "/Game/UI/Widget/WB_Ammo_Gain.WB_Ammo_Gain_C"))
    (UserInterface|Viewport|AddtoViewport _returnvalue 0)
    (if (or (<= (Variables|/Game/Blueprint/GameInstance/BP_Game_Instance.BP_Game_Instance_C|GetGun_reserve_Shotgun _as_bp_game_instance_10) _gun_max_munitions_shotgun) (<= (Variables|/Game/Blueprint/GameInstance/BP_Game_Instance.BP_Game_Instance_C|GetGun_reserve_SMG _as_bp_game_instance_10) _gun_max_munitions_smg_2))
      (if (and (<= (Variables|/Game/Blueprint/GameInstance/BP_Game_Instance.BP_Game_Instance_C|GetGun_reserve_Shotgun _as_bp_game_instance_2) (Variables|/Game/Blueprint/GameInstance/BP_Game_Instance.BP_Game_Instance_C|GetGun_Max_Munitions_Shotgun _as_bp_game_instance_2)) (<= (Variables|/Game/Blueprint/GameInstance/BP_Game_Instance.BP_Game_Instance_C|GetGun_reserve_SMG _as_bp_game_instance_2) (Variables|/Game/Blueprint/GameInstance/BP_Game_Instance.BP_Game_Instance_C|GetGun_Max_Munitions_SMG _as_bp_game_instance_2)))
        (Variables|/Game/Blueprint/GameInstance/BP_Game_Instance.BP_Game_Instance_C|SetGun_reserve_SMG _as_bp_game_instance_5 (Math|Float|Clamp(Float) (+ (Variables|/Game/Blueprint/GameInstance/BP_Game_Instance.BP_Game_Instance_C|GetGun_reserve_SMG _as_bp_game_instance_5) (Variables|InstanceEditable|GetQte_de_munitions_SMG)) 0.0 (Variables|/Game/Blueprint/GameInstance/BP_Game_Instance.BP_Game_Instance_C|GetGun_Max_reserve_SMG _as_bp_game_instance_5)))
        (Variables|/Game/Blueprint/GameInstance/BP_Game_Instance.BP_Game_Instance_C|SetGun_reserve_Shotgun _as_bp_game_instance_5 (Math|Float|Clamp(Float) (+ (Variables|/Game/Blueprint/GameInstance/BP_Game_Instance.BP_Game_Instance_C|GetGun_reserve_Shotgun _as_bp_game_instance_5) (Variables|InstanceEditable|GetQte_de_munitions_Shotgun)) 0.0 (Variables|/Game/Blueprint/GameInstance/BP_Game_Instance.BP_Game_Instance_C|GetGun_Max_reserve_Shotgun _as_bp_game_instance_5)))
        (Actor|DestroyActor)
        (Default|SetReserve (Variables|Static|GetAs%20BP%20First%20Person%20Character))
        (Actor|DestroyActor)
        (Default|SetReserve (Variables|Static|GetAs%20BP%20First%20Person%20Character))
        (elif (Math|Boolean|ANDBoolean (<= (Variables|/Game/Blueprint/GameInstance/BP_Game_Instance.BP_Game_Instance_C|GetGun_reserve_SMG _as_bp_game_instance_13) (Variables|/Game/Blueprint/GameInstance/BP_Game_Instance.BP_Game_Instance_C|GetGun_Max_Munitions_SMG _as_bp_game_instance_13)) (< (Variables|/Game/Blueprint/GameInstance/BP_Game_Instance.BP_Game_Instance_C|GetGun_reserve_Shotgun _as_bp_game_instance_13) (Variables|/Game/Blueprint/GameInstance/BP_Game_Instance.BP_Game_Instance_C|GetGun_Max_reserve_Shotgun _as_bp_game_instance_13)) (> (Variables|/Game/Blueprint/GameInstance/BP_Game_Instance.BP_Game_Instance_C|GetGun_reserve_Shotgun _as_bp_game_instance_13) (Variables|/Game/Blueprint/GameInstance/BP_Game_Instance.BP_Game_Instance_C|GetGun_Max_Munitions_Shotgun _as_bp_game_instance_13)))
          (Variables|/Game/Blueprint/GameInstance/BP_Game_Instance.BP_Game_Instance_C|SetGun_reserve_SMG _as_bp_game_instance_14 (Math|Float|Clamp(Float) (+ (Variables|/Game/Blueprint/GameInstance/BP_Game_Instance.BP_Game_Instance_C|GetGun_reserve_SMG _as_bp_game_instance_7) (Variables|InstanceEditable|GetQte_de_munitions_SMG)) 0.0 (Variables|/Game/Blueprint/GameInstance/BP_Game_Instance.BP_Game_Instance_C|GetGun_Max_reserve_SMG _as_bp_game_instance_7)))
          (Variables|/Game/Blueprint/GameInstance/BP_Game_Instance.BP_Game_Instance_C|SetGun_reserve_Shotgun _as_bp_game_instance_14 (Variables|/Game/Blueprint/GameInstance/BP_Game_Instance.BP_Game_Instance_C|GetGun_Max_reserve_Shotgun _as_bp_game_instance_14))
          (Actor|DestroyActor)
          (Default|SetReserve (Variables|Static|GetAs%20BP%20First%20Person%20Character))
          (elif (Math|Boolean|ANDBoolean (< (Variables|/Game/Blueprint/GameInstance/BP_Game_Instance.BP_Game_Instance_C|GetGun_reserve_SMG _as_bp_game_instance_4) (Variables|/Game/Blueprint/GameInstance/BP_Game_Instance.BP_Game_Instance_C|GetGun_Max_reserve_SMG _as_bp_game_instance_4)) (> (Variables|/Game/Blueprint/GameInstance/BP_Game_Instance.BP_Game_Instance_C|GetGun_reserve_SMG _as_bp_game_instance_4) (Variables|/Game/Blueprint/GameInstance/BP_Game_Instance.BP_Game_Instance_C|GetGun_Max_Munitions_SMG _as_bp_game_instance_4)) (<= (Variables|/Game/Blueprint/GameInstance/BP_Game_Instance.BP_Game_Instance_C|GetGun_reserve_Shotgun _as_bp_game_instance_4) (Variables|/Game/Blueprint/GameInstance/BP_Game_Instance.BP_Game_Instance_C|GetGun_Max_Munitions_Shotgun _as_bp_game_instance_4)))
            (Variables|/Game/Blueprint/GameInstance/BP_Game_Instance.BP_Game_Instance_C|SetGun_reserve_Shotgun _as_bp_game_instance_16 (Math|Float|Clamp(Float) (+ (Variables|/Game/Blueprint/GameInstance/BP_Game_Instance.BP_Game_Instance_C|GetGun_reserve_Shotgun _as_bp_game_instance_16) (Variables|InstanceEditable|GetQte_de_munitions_Shotgun)) 0.0 (Variables|/Game/Blueprint/GameInstance/BP_Game_Instance.BP_Game_Instance_C|GetGun_Max_reserve_Shotgun _as_bp_game_instance_16)))
            (Variables|/Game/Blueprint/GameInstance/BP_Game_Instance.BP_Game_Instance_C|SetGun_reserve_SMG _as_bp_game_instance_8 (Variables|/Game/Blueprint/GameInstance/BP_Game_Instance.BP_Game_Instance_C|GetGun_Max_reserve_SMG _as_bp_game_instance_8))
            (Actor|DestroyActor)
            (Default|SetReserve (Variables|Static|GetAs%20BP%20First%20Person%20Character))
            (else
              (if (Math|Boolean|ANDBoolean (< (Variables|/Game/Blueprint/GameInstance/BP_Game_Instance.BP_Game_Instance_C|GetGun_reserve_SMG _as_bp_game_instance_10) (Variables|/Game/Blueprint/GameInstance/BP_Game_Instance.BP_Game_Instance_C|GetGun_Max_reserve_SMG _as_bp_game_instance_10)) (> (Variables|/Game/Blueprint/GameInstance/BP_Game_Instance.BP_Game_Instance_C|GetGun_reserve_SMG _as_bp_game_instance_10) _gun_max_munitions_smg_2) (< (Variables|/Game/Blueprint/GameInstance/BP_Game_Instance.BP_Game_Instance_C|GetGun_reserve_Shotgun _as_bp_game_instance_10) (Variables|/Game/Blueprint/GameInstance/BP_Game_Instance.BP_Game_Instance_C|GetGun_Max_reserve_Shotgun _as_bp_game_instance_10)) (> (Variables|/Game/Blueprint/GameInstance/BP_Game_Instance.BP_Game_Instance_C|GetGun_reserve_Shotgun _as_bp_game_instance_10) _gun_max_munitions_shotgun)) :!label _label
                (Variables|/Game/Blueprint/GameInstance/BP_Game_Instance.BP_Game_Instance_C|SetGun_reserve_SMG _as_bp_game_instance_15 (Variables|/Game/Blueprint/GameInstance/BP_Game_Instance.BP_Game_Instance_C|GetGun_Max_reserve_SMG _as_bp_game_instance_15))
                (Variables|/Game/Blueprint/GameInstance/BP_Game_Instance.BP_Game_Instance_C|SetGun_reserve_Shotgun _as_bp_game_instance_15 (Variables|/Game/Blueprint/GameInstance/BP_Game_Instance.BP_Game_Instance_C|GetGun_Max_reserve_Shotgun _as_bp_game_instance_15))
                (Actor|DestroyActor)
                (Default|SetReserve (Variables|Static|GetAs%20BP%20First%20Person%20Character))
                (else
                  ;[1 1 1] SMG utilisé mais pas le shotgun
                  (if (and (== (Variables|/Game/Blueprint/GameInstance/BP_Game_Instance.BP_Game_Instance_C|GetGun_reserve_Shotgun _as_bp_game_instance_3) (Variables|/Game/Blueprint/GameInstance/BP_Game_Instance.BP_Game_Instance_C|GetGun_Max_reserve_Shotgun _as_bp_game_instance_3)) (<= (Variables|/Game/Blueprint/GameInstance/BP_Game_Instance.BP_Game_Instance_C|GetGun_reserve_SMG _as_bp_game_instance_3) _gun_max_munitions_smg))
                    (Variables|/Game/Blueprint/GameInstance/BP_Game_Instance.BP_Game_Instance_C|SetGun_reserve_SMG _as_bp_game_instance_6 (+ (Variables|/Game/Blueprint/GameInstance/BP_Game_Instance.BP_Game_Instance_C|GetGun_reserve_SMG _as_bp_game_instance_6) (Variables|InstanceEditable|GetQte_de_munitions_SMG)))
                    (Actor|DestroyActor)
                    (Default|SetReserve (Variables|Static|GetAs%20BP%20First%20Person%20Character))
                    (elif (Math|Boolean|ANDBoolean (< (Variables|/Game/Blueprint/GameInstance/BP_Game_Instance.BP_Game_Instance_C|GetGun_reserve_SMG _as_bp_game_instance_3) (Variables|/Game/Blueprint/GameInstance/BP_Game_Instance.BP_Game_Instance_C|GetGun_Max_reserve_SMG _as_bp_game_instance_3)) (> (Variables|/Game/Blueprint/GameInstance/BP_Game_Instance.BP_Game_Instance_C|GetGun_reserve_SMG _as_bp_game_instance_3) _gun_max_munitions_smg) (== (Variables|/Game/Blueprint/GameInstance/BP_Game_Instance.BP_Game_Instance_C|GetGun_reserve_Shotgun _as_bp_game_instance_3) (Variables|/Game/Blueprint/GameInstance/BP_Game_Instance.BP_Game_Instance_C|GetGun_Max_reserve_Shotgun _as_bp_game_instance_3)))
                      (Variables|/Game/Blueprint/GameInstance/BP_Game_Instance.BP_Game_Instance_C|SetGun_reserve_SMG _as_bp_game_instance_17 (Variables|/Game/Blueprint/GameInstance/BP_Game_Instance.BP_Game_Instance_C|GetGun_Max_reserve_SMG _as_bp_game_instance_17))
                      (Actor|DestroyActor)
                      (Default|SetReserve (Variables|Static|GetAs%20BP%20First%20Person%20Character))
                      (else
                        ;[1 1 1] Si le Shotgun a été utilisé mais pas le SMG
                        (if (Math|Boolean|ANDBoolean (<= (Variables|/Game/Blueprint/GameInstance/BP_Game_Instance.BP_Game_Instance_C|GetGun_reserve_Shotgun _as_bp_game_instance) _gun_max_reserve_shotgun) (== (Variables|/Game/Blueprint/GameInstance/BP_Game_Instance.BP_Game_Instance_C|GetGun_reserve_SMG _as_bp_game_instance) (Variables|/Game/Blueprint/GameInstance/BP_Game_Instance.BP_Game_Instance_C|GetGun_reserve_SMG _as_bp_game_instance)) (>= (Variables|/Game/Blueprint/GameInstance/BP_Game_Instance.BP_Game_Instance_C|GetGun_reserve_Shotgun _as_bp_game_instance) (- _gun_max_reserve_shotgun _gun_max_munitions_shotgun_2)))
                          (Variables|/Game/Blueprint/GameInstance/BP_Game_Instance.BP_Game_Instance_C|SetGun_reserve_Shotgun _as_bp_game_instance_9 (Variables|/Game/Blueprint/GameInstance/BP_Game_Instance.BP_Game_Instance_C|GetGun_Max_reserve_Shotgun _as_bp_game_instance_9))
                          (Actor|DestroyActor)
                          (Default|SetReserve (Variables|Static|GetAs%20BP%20First%20Person%20Character))
                          (elif (Math|Boolean|ANDBoolean (== (Variables|/Game/Blueprint/GameInstance/BP_Game_Instance.BP_Game_Instance_C|GetGun_reserve_SMG _as_bp_game_instance) (Variables|/Game/Blueprint/GameInstance/BP_Game_Instance.BP_Game_Instance_C|GetGun_reserve_SMG _as_bp_game_instance)) (< (Variables|/Game/Blueprint/GameInstance/BP_Game_Instance.BP_Game_Instance_C|GetGun_reserve_Shotgun _as_bp_game_instance) _gun_max_reserve_shotgun) (> (Variables|/Game/Blueprint/GameInstance/BP_Game_Instance.BP_Game_Instance_C|GetGun_reserve_Shotgun _as_bp_game_instance) _gun_max_munitions_shotgun_2))
                            (Variables|/Game/Blueprint/GameInstance/BP_Game_Instance.BP_Game_Instance_C|SetGun_reserve_Shotgun _as_bp_game_instance_12 (+ (Variables|/Game/Blueprint/GameInstance/BP_Game_Instance.BP_Game_Instance_C|GetGun_reserve_Shotgun _as_bp_game_instance_12) (Variables|InstanceEditable|GetQte_de_munitions_Shotgun)))
                            (Actor|DestroyActor)
                            (Default|SetReserve (Variables|Static|GetAs%20BP%20First%20Person%20Character))
                            (else
                              (Variables|/Game/Blueprint/GameInstance/BP_Game_Instance.BP_Game_Instance_C|SetGun_reserve_SMG _as_bp_game_instance_11 (Variables|/Game/Blueprint/GameInstance/BP_Game_Instance.BP_Game_Instance_C|GetGun_Max_reserve_SMG _as_bp_game_instance_11))
                              (Variables|/Game/Blueprint/GameInstance/BP_Game_Instance.BP_Game_Instance_C|SetGun_reserve_Shotgun _as_bp_game_instance_11 (Variables|/Game/Blueprint/GameInstance/BP_Game_Instance.BP_Game_Instance_C|GetGun_Max_reserve_Shotgun _as_bp_game_instance_11))
                              (Actor|DestroyActor)
                              (Default|SetReserve (Variables|Static|GetAs%20BP%20First%20Person%20Character))))))))))))))
      (else
        (goto _label)))))

(event EventBeginPlay
  ;[1 1 1] Begin play
  (bind _asbp_first_person_character (Utilities|Casting|CastToBP_FirstPersonCharacter (Game|GetPlayerCharacter 0)))
  (Variables|Static|SetAs%20BP%20First%20Person%20Character _asbp_first_person_character)
  (bind _asbp_game_instance (Utilities|Casting|CastToBP_Game_Instance (Game|GetGameInstance)))
  (Variables|Static|SetAs%20BP%20Game%20Instance _asbp_game_instance))

(fn ConstructionScript)